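; BP_TimerTagManager is a trigger actor that runs a one-time countdown once BP_Character enters its box.
; The first overlap creates the TimerUI widget and starts a looping timer that decrements Seconds and updates the display.
; At zero it spawns a scaled-down Bp_Memory above itself, destroys the BP_AIBlutter actors cached at BeginPlay and clears the timer within that loop.
; Minute rollover and sound nodes are disconnected, so Minutes is display-only.
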(event `self.ReceiveBeginPlay`
  (bind _outactors (`GameplayStatics.GetAllActorsOfClass` "/Game/Blueprints/AI/BP_AIBlutter.BP_AIBlutter_C"))
  (set `self.CharsAi` _outactors))

(event `self.Box.OnComponentBeginOverlap`
  (params (OverlappedComponent :type "PrimitiveComponent Object Reference") (OtherActor :type "Actor Object Reference") (OtherComp :type "PrimitiveComponent Object Reference") (OtherBodyIndex :type Integer) (bFromSweep :type Boolean) (SweepResult :type "HitResult Structure (by ref)"))
  (cast `/Game/Blueprints/Character/BP_Character` OtherActor)
  (if (not (`self.Entered`))
    (set `self.Entered` true)
    (cast `/Game/Blueprints/Character/BP_Character` OtherActor)
    (bind _returnvalue (`|CreateWidget` "/Game/UI/TimerUI.TimerUI_C"))
    (bind _output_get (set `self.UI` _returnvalue))
    (`UserWidget.AddToViewport` _output_get 0)
    (`KismetSystemLibrary.K2_SetTimer` null "StartTimer" 1.0 true)
    (`/Game/UI/TimerUI.SetSeconds` (`self.UI`) (`KismetTextLibrary.Conv_IntToText` (`self.Seconds`)))
    (`/Game/UI/TimerUI.SetMinutes` (`self.UI`) (`KismetTextLibrary.Conv_IntToText` (`self.Minutes`)))))

(event `StartTimer`
  (bind _returnvalue (`self.GetTransform`))
  (if (== (`self.Seconds`) 0)
    (`|SpawnActorFromClass` "/Game/Blueprints/Objects/Bp_Memory.Bp_Memory_C" (`KismetMathLibrary.MakeTransform` (`KismetMathLibrary.MakeVector` (.x (.location _returnvalue)) (.y (.location _returnvalue)) (+ (.z (.location _returnvalue)) 10.0)) (.rotation _returnvalue) (* (.scale _returnvalue) 0.15)) "Undefined" "MultiplyWithRoot" null null)
    (for _array_element (`self.CharsAi`)
      (`self.K2_DestroyActor` _array_element)
      (`KismetSystemLibrary.K2_ClearTimer` null "StartTimer"))
    (else
      (bind _output_get (set `self.Seconds` (- (`self.Seconds`) 1)))
      (`/Game/UI/TimerUI.SetSeconds` (`self.UI`) (`KismetTextLibrary.Conv_IntToText` _output_get)))))

(fn `UserConstructionScript`)