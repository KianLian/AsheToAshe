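; Physics door that the player grabs and swings with look input, with an optional exit-door mode.
; Grabbing locks movement and camera look, then turns look input into door yaw, flipped by the player's side; releasing restores control.
; Exit doors start with physics off until the game mode permits leaving.
; A character entering the trigger box snaps the door shut, makes it extremely heavy and blocks further grabs.
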(event `self.ReceiveBeginPlay`
  (set `self.Relative Rotation` (`SceneComponent.RelativeRotation` (`self.Door`)))
  (set `self.PlayerRef` (`GameplayStatics.GetPlayerCharacter` 0))
  (if (`self.IsToLeave`)
    (`PrimitiveComponent.SetSimulatePhysics` (`self.Door`) false)))

(event `DoorToLeave`
  (params (Bah :type "Actor Object Reference")))

(event `EnhancedInput|/Game/Blueprints/Character/Input/Actions/IA_Look`
  (params (ActionValue :type "Vector2D Structure") (ElapsedSeconds :type "Float (double-precision)") (TriggeredSeconds :type "Float (double-precision)") (InputAction :type "InputAction Object Reference" :default "/Game/Blueprints/Character/Input/Actions/IA_Look.IA_Look"))
  (bind (_x _y) (`KismetMathLibrary.BreakVector2D` ActionValue))
  ;[1 1 1] Inputs
  (:`Triggered`
    (`self.MoveDoor` _x)
    (`self.MoveDoor` _y)
    (`/Engine/EditorBlueprintResources/StandardMacros.DoOnce` false :!label _label
      (:`Completed`
        (`GameplayStatics.PlaySoundAtLocation` "/Game/sounds/OpenDoor.OpenDoor" (`self.K2_GetActorLocation`) (struct) 1.0 1.0 0.0 null null null null)))))

(event `/Game/Blueprints/Interfaces/BPI_Grabble.GrabObject`
  (bind _returnvalue (`GameplayStatics.GetPlayerController` 0))
  ;[1 1 1] GrabObject
  (if (not (`self.DoorClosed`))
    (if (not (`self.DoorPlayerOpen`))
      (if (`self.IsToLeave`)
        (bind _asbp_game_mode (cast `/Game/Blueprints/Modes/BP_GameMode` (`GameplayStatics.GetGameMode`)))
        (bind _canleave (`/Game/Blueprints/Modes/BP_GameMode.CanLeaveTheArea` _asbp_game_mode))
        (if _canleave
          (`PrimitiveComponent.SetSimulatePhysics` (`self.Door`) true)
          (`CharacterMovementComponent.DisableMovement` (`Character.CharacterMovement` (`self.PlayerRef`)) :!label _label_2)
          (`Controller.SetIgnoreLookInput` _returnvalue true)
          (`self.EnableInput` _returnvalue)))
      (else
        (goto _label_2)))))

(event `/Game/Blueprints/Interfaces/BPI_Grabble.ReleaseObject`
  (bind _returnvalue (`GameplayStatics.GetPlayerController` 0))
  (bind _playerref (`self.PlayerRef`))
  ;[1 1 1] Release Obejct
  (`self.DisableInput` _returnvalue)
  (`Controller.ResetIgnoreLookInput` _returnvalue)
  (`self.EnableInput` _playerref _returnvalue)
  (`CharacterMovementComponent.SetMovementMode` (`Character.CharacterMovement` _playerref) "MOVE_Walking" 0)
  (goto _label :!via `Reset`))

(event `MoveDoor`
  (params (Amout :type "Float (double-precision)"))
  (bind _door (`self.Door`))
  ;[1 1 1] Move Door
  (`SceneComponent.K2_SetRelativeRotation` _door (`KismetMathLibrary.ComposeRotators` (`SceneComponent.RelativeRotation` _door) (`KismetMathLibrary.MakeRotator` 0.0 0.0 (* Amout (`KismetMathLibrary.SelectFloat` -1.0 1.0 (>= (`KismetMathLibrary.Dot_VectorVector` (`KismetMathLibrary.Normal` (- (`self.K2_GetActorLocation`) (`self.K2_GetActorLocation` (`self.PlayerRef`)))) (`self.GetActorForwardVector`)) 0.0))))) false false))

(event `self.Box.OnComponentBeginOverlap`
  (params (OverlappedComponent :type "PrimitiveComponent Object Reference") (OtherActor :type "Actor Object Reference") (OtherComp :type "PrimitiveComponent Object Reference") (OtherBodyIndex :type Integer) (bFromSweep :type Boolean) (SweepResult :type "HitResult Structure (by ref)"))
  ;[1 1 1] Box To Close
  (if (and (`.bSuccess` (cast `/Game/Blueprints/Character/BP_Character` OtherActor :!pure true)) (not (`self.DoorClosed`)))
    (`SceneComponent.K2_SetRelativeRotation` (`self.Door`) (`self.Relative Rotation`) false true)
    (set `self.DoorClosed` true)
    (`PrimitiveComponent.SetMassScale` (`self.Door`) "None" 1000000000.0)
    (`GameplayStatics.PlaySoundAtLocation` "/Game/sounds/__close_door_Cue.__close_door_Cue" (`self.K2_GetActorLocation`) (struct) 1.0 1.0 0.0 null null null null)))

(fn `UserConstructionScript`)